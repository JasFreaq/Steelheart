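; Actor component for cursor-driven slicing of destructible objects in a test setup.
; While slicing, cursor traces track entry and current points per hit component; release or leaving it attempts a cut if the stroke is long enough relative to its bounds.
; The cut plane comes from the stroke and owner location.
; Non-procedural targets are replaced by BP_ProcMesh, then sliced with caps; the new half simulates physics and receives a radial impulse.
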(event Custom|Begin%20Slice
  (bind _returnvalue (Game|GetPlayerController 0))
  (bind _array (Utilities|Array|MakeArray "ObjectTypeQuery7" "ObjectTypeQuery6"))
  (bind (_hitresult _returnvalue_2) (Class|PlayerController|GetHitResultUnderCursorforObjects _returnvalue _array false))
  (bind (_bblockinghit _binitialoverlap _time _distance _location _impactpoint _normal _impactnormal _physmat _hitactor _hitcomponent) (Collision|BreakHitResult _hitresult))
  (Variables|Default|SetIsSlicing true)
  (if _returnvalue_2
    (CallFunction|SetSliceStartVariables _hitactor _hitcomponent _impactpoint)
    (Development|PrintString (Utilities|GetDisplayName _hitcomponent))))

(event Custom|End%20Slice
  (Variables|Default|SetIsSlicing false)
  (bind _valid (CallFunction|SetSliceVariables))
  (if _valid
    (CallFunction|TrySlice))
  (CallFunction|SetSliceStartVariables 0 0 "0, 0, 0"))

(event Custom|Try%20Slice
  (bind _slice_actor (Variables|Default|GetSlice%20Actor))
  (Utilities|IsValid _slice_actor
    (:Is%20Valid
      (bind _asprocedural_mesh_component (Utilities|Casting|CastToProceduralMeshComponent (Variables|Default|GetSlice%20Component))
        (:then
          (CallFunction|SliceMesh _asprocedural_mesh_component))
        (:CastFailed
          (bind _returnvalue (Game|SpawnActorfromClass "/Game/_Game/Test/BP_ProcMesh.BP_ProcMesh_C" (Transformation|GetActorTransform _slice_actor) "Undefined" 0 0))
          (bind _new_proc_mesh (Default|SetupProcMesh _returnvalue (Variables|/Script/Engine.StaticMeshComponent|GetStaticMesh (Actor|GetComponentbyClass _slice_actor "/Script/Engine.StaticMeshComponent"))))
          (Actor|DestroyActor (Variables|Default|GetSlice%20Actor))
          (CallFunction|SliceMesh _new_proc_mesh))))))

(event Custom|Slice%20Mesh
  (params (ProcMesh :type Procedural%20Mesh%20Component%20Object%20Reference))
  (bind _radialforce (Variables|Default|GetRadialForce))
  (bind _slice_position (Variables|Default|GetSlice%20Position))
  (bind _outotherhalfprocmesh (Class|KismetProceduralMeshLibrary|SliceProceduralMesh ProcMesh _slice_position (Variables|Default|GetSlice%20Normal) true "CreateNewSectionForCap" "/Game/StarterContent/Materials/M_Metal_Brushed_Nickel.M_Metal_Brushed_Nickel"))
  (Physics|SetSimulatePhysics _outotherhalfprocmesh true)
  (Collision|SetCollisionObjectType _outotherhalfprocmesh "ECC_GameTraceChannel1")
  (Transformation|SetWorldLocation _radialforce _slice_position false false)
  (Class|RadialForceComponent|FireImpulse _radialforce))

(event Custom|Update%20Slice
  (bind _returnvalue (Game|GetPlayerController 0))
  (bind _array (Utilities|Array|MakeArray "ObjectTypeQuery7" "ObjectTypeQuery6"))
  (bind (_hitresult _returnvalue_2) (Class|PlayerController|GetHitResultUnderCursorforObjects _returnvalue _array false))
  (bind (_bblockinghit _binitialoverlap _time _distance _location _impactpoint _normal _impactnormal _physmat _hitactor _hitcomponent) (Collision|BreakHitResult _hitresult))
  (if (Variables|Default|GetIsSlicing)
    (if _returnvalue_2
      (Development|PrintString (Utilities|GetDisplayName _hitcomponent))
      (Utilities|IsValid (Variables|Default|GetSlice%20Actor)
        (:Is%20Valid
          (Variables|Default|SetRaycast%20Current _impactpoint)
          (if (!= (Variables|Default|GetSlice%20Actor) _hitactor)
            (bind _valid (CallFunction|SetSliceVariables :!label _label))
            (if _valid
              (CallFunction|TrySlice))
            (CallFunction|SetSliceStartVariables _hitactor _hitcomponent _impactpoint)
            (elif (!= (Variables|Default|GetSlice%20Component) _hitcomponent)
              (goto _label))))
        (:Is%20Not%20Valid
          (CallFunction|SetSliceStartVariables _hitactor _hitcomponent _impactpoint)))
      (else
        (Development|PrintString (Utilities|GetDisplayName _hitcomponent))
        (bind _valid_2 (CallFunction|SetSliceVariables))
        (if _valid_2
          (CallFunction|TrySlice))
        (CallFunction|SetSliceStartVariables 0 0 "0, 0, 0")))))

(fn CalculatePlaneNormal
  (params (B :type Vector) (A :type Vector))
  (return (Math|Vector|Normalize (Math|Vector|CrossProduct (- B A) (- (Transformation|GetActorLocation (Components|GetOwner)) A)))))

(fn SetSliceStartVariables
  (params (Slice%20Actor :type Actor%20Object%20Reference) (Slice%20Component :type Primitive%20Component%20Object%20Reference) (Hit%20Position :type Vector))
  (Variables|Default|SetSlice%20Actor Slice%20Actor)
  (Variables|Default|SetSlice%20Component Slice%20Component)
  (Variables|Default|SetRaycast%20Start Hit%20Position)
  (Variables|Default|SetRaycast%20Current Hit%20Position))

(fn SetSliceVariables
  (if (>= (/ (Math|Vector|Distance(Vector) (Variables|Default|GetRaycast%20Start) (Variables|Default|GetRaycast%20Current)) (* (Math|Vector|VectorLength (.BoxExtent (Collision|GetComponentBounds (Variables|Default|GetSlice%20Component)))) 2.0)) (Variables|Default|GetSliceRatio))
    (Variables|Default|SetSlice%20Position (/ (+ (Variables|Default|GetRaycast%20Start) (Variables|Default|GetRaycast%20Current)) (Variables|Default|GetPosDividend)))
    (Variables|Default|SetSlice%20Normal (CallFunction|CalculatePlaneNormal (Variables|Default|GetRaycast%20Current) (Variables|Default|GetRaycast%20Start)))
    (return true)
    (else
      (return false))))