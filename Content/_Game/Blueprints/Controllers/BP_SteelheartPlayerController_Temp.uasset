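; Player controller for Steelheart that fires a mouse-aimed slicing laser from the player's head socket while right mouse is held.
; A lazily spawned, reused BP_RayTester aims at the cursor hit or deprojected direction, stretching to the distance and smoothing yaw and roll while pitch snaps.
; BPSlicerComp begins, updates and ends slices alongside the ray.
; Aiming outside LaserFrustrumAngle from the character's forward vector deactivates the laser.
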(event Custom|Deactivate%20Laser
  (bind _ray (Variables|Default|GetRay))
  (Variables|Default|SetRayActive false)
  (Utilities|IsValid _ray
    (:Is%20Valid
      (Rendering|SetVisibility (Variables|/Script/Engine.Character|GetCapsuleComponent _ray) false true)
      (Default|EndSlice (Variables|Default|GetBP_SlicerComp)))))

(event EventBeginPlay
  (Variables|/Game/_Game/Test/BP_SlicerComp.BP_SlicerComp_C|SetRadialForce (Variables|Default|GetBP_SlicerComp) (Variables|Default|GetRadialForce)))

(event EventTick
  (params (DeltaSeconds :type Float%20%28single-precision%29))
  (bind (_locationx _locationy) (Game|Player|GetMousePosition))
  (bind (_hitresult _returnvalue) (Game|Player|GetHitResultUnderCursorbyChannel "TraceTypeQuery1" false))
  (if (Variables|Default|GetRayActive)
    (Utilities|IsValid (Variables|Default|GetRay)
      (:Is%20Valid
        (if _returnvalue
          (CallFunction|UpdateRayAngle (.Location (Collision|BreakHitResult _hitresult)))
          (else
            (CallFunction|UpdateRayAngle (+ (Transformation|GetSocketLocation (Variables|/Script/Engine.Character|GetMesh (Game|GetPlayerCharacter 0)) "headSocket") (* (.WorldDirection (Class|GameplayStatics|DeprojectScreentoWorld self (Math|Vector2D|MakeVector2D _locationx _locationy))) 1e+04)))))))))

(event Input|MouseEvents|RightMouseButton
  (params (Key :type Key%20Structure :default "None"))
  (bind (_locationx _locationy) (Game|Player|GetMousePosition))
  (:Pressed
    (Variables|Default|SetRayActive true)
    (Default|BeginSlice (Variables|Default|GetBP_SlicerComp))
    (Utilities|IsValid (Variables|Default|GetRay)
      (:Is%20Valid
        (Rendering|SetVisibility (Variables|/Script/Engine.Character|GetCapsuleComponent (Variables|Default|GetRay)) true true))
      (:Is%20Not%20Valid
        (bind _returnvalue (Game|SpawnActorfromClass "/Game/_Game/Test/Fx/BP_RayTester.BP_RayTester_C" (Math|Transform|MakeTransform "0, 0, 0") "Undefined" 0 0))
        (bind _output_get (Variables|Default|SetRay _returnvalue))
        (Transformation|AttachComponentToComponent _output_get (Variables|/Script/Engine.Character|GetMesh (Game|GetPlayerCharacter 0)) "headSocket" "SnapToTarget" "SnapToTarget" "SnapToTarget" false)))
    (CallFunction|SetRayAngle (+ (Transformation|GetSocketLocation (Variables|/Script/Engine.Character|GetMesh (Game|GetPlayerCharacter 0)) "headSocket") (* (.WorldDirection (Class|GameplayStatics|DeprojectScreentoWorld self (Math|Vector2D|MakeVector2D _locationx _locationy))) 1e+03))))
  (:Released
    (CallFunction|DeactivateLaser)))

(fn ConstructionScript)

(fn SetRayAngle
  (params (End%20Location :type Vector))
  (bind _returnvalue (Game|GetPlayerCharacter 0))
  (bind _ray (Variables|Default|GetRay))
  (bind _ray_2 (Variables|/Game/_Game/Test/Fx/BP_RayTester.BP_RayTester_C|GetRay _ray))
  (bind _returnvalue_2 (Transformation|GetWorldScale _ray_2))
  (LocalVariables|SetSocket%20Location (Transformation|GetSocketLocation (Variables|/Script/Engine.Character|GetMesh _returnvalue) "headSocket"))
  (if (<= (Math|Float|Absolute(Float) (Class|KismetMathLibrary|DegAcos (Math|Vector|DotProduct (Math|Vector|Normalize (Math|Vector|GetForwardVector (Variables|/Script/Engine.Actor|GetRootComponent _returnvalue))) (Math|Vector|Normalize (- End%20Location (LocalVariables|GetSocket%20Location)))))) (Variables|Default|GetLaserFrustrumAngle))
    (Transformation|SetWorldScale3D _ray_2 (Math|Vector|MakeVector (/ (Math|Vector|Distance(Vector) (LocalVariables|GetSocket%20Location) End%20Location) (Variables|Default|GetRayLengthRatio)) (.y _returnvalue_2) (.z _returnvalue_2)))
    (Transformation|SetWorldRotation _ray_2 (Math|Rotator|FindLookatRotation (LocalVariables|GetSocket%20Location) End%20Location) false false)
    (Default|UpdateSlice (Variables|Default|GetBP_SlicerComp))
    (else
      (CallFunction|DeactivateLaser))))

(fn UpdateRayAngle
  (params (End%20Location :type Vector))
  (bind _returnvalue (Game|GetPlayerCharacter 0))
  (bind _ray (Variables|Default|GetRay))
  (bind _ray_2 (Variables|/Game/_Game/Test/Fx/BP_RayTester.BP_RayTester_C|GetRay _ray))
  (bind _returnvalue_2 (Transformation|GetWorldScale _ray_2))
  (LocalVariables|SetSocket%20Location (Transformation|GetSocketLocation (Variables|/Script/Engine.Character|GetMesh _returnvalue) "headSocket"))
  (if (<= (Math|Float|Absolute(Float) (Class|KismetMathLibrary|DegAcos (Math|Vector|DotProduct (Math|Vector|Normalize (Math|Vector|GetForwardVector (Variables|/Script/Engine.Actor|GetRootComponent _returnvalue))) (Math|Vector|Normalize (- End%20Location (LocalVariables|GetSocket%20Location)))))) (Variables|Default|GetLaserFrustrumAngle))
    (Transformation|SetWorldScale3D _ray_2 (Math|Vector|MakeVector (/ (Math|Vector|Distance(Vector) (LocalVariables|GetSocket%20Location) End%20Location) (Variables|Default|GetRayLengthRatio)) (.y _returnvalue_2) (.z _returnvalue_2)))
    (Transformation|SetWorldRotation _ray_2 (Math|Rotator|MakeRotator (.roll (Math|Interpolation|RInterpTo (Transformation|GetWorldRotation (Variables|/Game/_Game/Test/Fx/BP_RayTester.BP_RayTester_C|GetRay (Variables|Default|GetRay))) (Math|Rotator|FindLookatRotation (LocalVariables|GetSocket%20Location) End%20Location) (Utilities|Time|GetWorldDeltaSeconds) 5.0)) (.Pitch (Math|Rotator|BreakRotator (Math|Rotator|FindLookatRotation (LocalVariables|GetSocket%20Location) End%20Location))) (.yaw (Math|Interpolation|RInterpTo (Transformation|GetWorldRotation (Variables|/Game/_Game/Test/Fx/BP_RayTester.BP_RayTester_C|GetRay (Variables|Default|GetRay))) (Math|Rotator|FindLookatRotation (LocalVariables|GetSocket%20Location) End%20Location) (Utilities|Time|GetWorldDeltaSeconds) 5.0))) false false)
    (Default|UpdateSlice (Variables|Default|GetBP_SlicerComp))
    (else
      (CallFunction|DeactivateLaser))))